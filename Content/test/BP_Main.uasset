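; BP_Main is a test Blueprint that builds and initializes a grid of BP_Land tiles.
; The Ev_Spawn event spawns an 8x8 grid of tiles at 300-unit spacing, with no caller in this graph.
; One second after BeginPlay, it gathers every BP_Land, sets IsRoad and calls EvAni on each.
; The IsRoad check searches the array being iterated, so it marks every tile as road.
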(event Custom|Ev_Spawn
  (for _index (range 0 7)
    (for _index_2 (range 0 7)
      (Game|SpawnActorfromClass "/Game/test/BP_Land.BP_Land_C" (Math|Transform|MakeTransform (Math|Vector|MakeVector (Math|Conversions|ToFloat(Integer) (* _index 300)) (Math|Conversions|ToFloat(Integer) (* _index_2 300)) 0.0) "0, 0, 0" "1.000000,1.000000,1.000000") "Undefined" "MultiplyWithRoot" 0 0))))

(event EventBeginPlay
  (Utilities|FlowControl|Delay 1.0)
  (bind _outactors (Actor|GetAllActorsOfClass "/Game/test/BP_Land.BP_Land_C"))
  (for _array_element _outactors
    (Variables|/Game/test/BP_Land.BP_Land_C|SetIsRoad _array_element (!= (Utilities|Array|FindItem _outactors _array_element) -1))
    (Default|EvAni _array_element)))

(fn ConstructionScript)