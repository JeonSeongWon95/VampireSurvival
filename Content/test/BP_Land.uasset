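; BP_Land is a land tile that animates between road and wooded terrain states when Ev_Ani fires.
; A delay proportional to the tile's distance from the world origin staggers the change, so multiple tiles would update as an outward wave.
; IsRoad drives a material parameter, clears or sets the tree mesh, and picks a flat or random target height.
; A timeline lerps the land mesh to that height, then stores it as the next start.
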(event Custom|Ev_Ani
  (Utilities|FlowControl|Delay (* (Math|Vector|Distance(Vector) "0, 0, 0" (Transformation|GetActorLocation)) 5e-05))
  (if (Variables|Default|GetIsRoad)
    ;[1 1 1] Land Color
    (Rendering|Material|SetScalarParameterValueonMaterials (Variables|Default|GetSm_cube_land) "IsRoad" 1.0)
    ;[1 1 1] Tree Object
    (Components|StaticMesh|SetStaticMesh (Variables|Default|GetSm_cube_wood) 0)
    (Variables|Default|SetB 0.0)
    (bind _newtrack_0 (Timeline|Timeline PlayFromStart)
      (:Update
        (Transformation|SetRelativeLocation (Variables|Default|GetSm_cube_land) (Math|Vector|MakeVector 0.0 0.0 (Math|Float|Lerp (Variables|Default|GetA) (Variables|Default|GetB) _newtrack_0)) false false))
      (:Finished
        (Variables|Default|SetA (Variables|Default|GetB))))
    (else
      (Rendering|Material|SetScalarParameterValueonMaterials (Variables|Default|GetSm_cube_land) "IsRoad" 0.0)
      (Components|StaticMesh|SetStaticMesh (Variables|Default|GetSm_cube_wood) "/Game/test/Sm_cube_wood.Sm_cube_wood")
      (Variables|Default|SetB (Math|Random|RandomFloatinRange 0.0 5e+01))
      (Timeline|Timeline PlayFromStart))))

(fn ConstructionScript)